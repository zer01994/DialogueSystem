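; PC_Player is the player controller that switches between gameplay and dialogue or inventory UI, plus a language toggle.
; Dialogue show and hide events toggle the cursor and pawn input and message the pawn, with hiding also sending a camera switch and restoring game-only input.
; The Inventory action flip-flops a HUD inventory message with the same cursor and input handling.
; The L key flip-flops the culture between English and Russian.
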(event EventBeginPlay)

(event EventTick
  (params (DeltaSeconds :type Float%20%28single-precision%29)))

(event EventHideDialogueBox
  (bind _returnvalue (Pawn|GetControlledPawn))
  (bind _self self)
  (Variables|Default|SetbShowMouseCursor false)
  (Input|EnableInput _returnvalue _self)
  (Class|ICamera|SwitchCamera(Message) _returnvalue true)
  (Class|IPlayerControl|HideDialogueBox(Message) _returnvalue)
  (Input|SetInputModeGameOnly _self))

(event EventShowDialogueBox
  (bind _returnvalue (Pawn|GetControlledPawn))
  (Variables|Default|SetbShowMouseCursor true)
  (Input|DisableInput _returnvalue self)
  (Class|IPlayerControl|ShowDialogueBox(Message) _returnvalue))

(event Input|ActionEvents|InputActionInventory
  (params (Key :type Key%20Structure :default "None"))
  (bind _returnvalue (Pawn|GetControlledPawn))
  (bind _returnvalue_2 (HUD|GetHUD))
  (bind _self self)
  (:Pressed
    (Utilities|FlowControl|FlipFlop
      (:A
        (Class|IInventory|InventorySwitcher(Message) _returnvalue_2 true)
        (Variables|Default|SetbShowMouseCursor true)
        (Input|DisableInput _returnvalue _self))
      (:B
        (Class|IInventory|InventorySwitcher(Message) _returnvalue_2 false)
        (Variables|Default|SetbShowMouseCursor false)
        (Input|EnableInput _returnvalue _self)
        (Input|SetInputModeGameOnly _self)))))

(event Input|KeyboardEvents|L
  (params (Key :type Key%20Structure :default "None"))
  (:Pressed
    (Utilities|FlowControl|FlipFlop
      (:A
        (Class|KismetInternationalizationLibrary|SetCurrentCulture "en"))
      (:B
        (Class|KismetInternationalizationLibrary|SetCurrentCulture "ru")))))

(fn ConstructionScript)