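; In-game state object that tracks the player's evidence and checks it against the current level's success list.
; On BeginPlay it looks up the level name in DT_SuccessListEvidence and stores the required evidence count.
; Add ignores repeated keys, expands each DT_LevelListEvidence row into AllEvidenceList and sends each item to the HUD as a message.
; RefreshList replaces EvidenceList and compares it to the success row, only printing the result.
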(event Custom|CheckList
  (bind _returnvalue (Game|GetCurrentLevelName true))
  (bind _returnvalue_2 (Utilities|GetDataTableRow "/Game/Assets/DataTables/EvidenceDT/DT_SuccessListEvidence.DT_SuccessListEvidence" (Utilities|String|StringToName _returnvalue))
    (:then
      (if (Utilities|Array|Identical (Utilities|Struct|BreakS_SuccessListEvidence _returnvalue_2) (Variables|Default|GetEvidenceList))
        (Development|PrintString "true")
        (else
          (Development|PrintString "faaaalse"))))
    (:RowNotFound
      (Development|PrintString "GS_InGame RowNotFound"))))

(event Custom|GetCountSuccessListEvidence
  (bind _returnvalue (Game|GetCurrentLevelName true))
  (bind _returnvalue_2 (Utilities|GetDataTableRow "/Game/Assets/DataTables/EvidenceDT/DT_SuccessListEvidence.DT_SuccessListEvidence" (Utilities|String|StringToName _returnvalue))
    (:then
      (Variables|Default|SetSuccessListEvidenceCount (Utilities|Array|Length (Utilities|Struct|BreakS_SuccessListEvidence _returnvalue_2))))))

(event EventBeginPlay
  (CallFunction|GetCountSuccessListEvidence))

(event EventTick
  (params (DeltaSeconds :type Float%20%28single-precision%29)))

(event EventAdd
  (params (DT_LevelListEvidence :type String))
  (if (== (Utilities|Array|FindItem (Variables|Default|GetAddedEvidence) DT_LevelListEvidence) -1)
    (Utilities|Array|Add (Variables|Default|GetAddedEvidence) DT_LevelListEvidence)
    (bind _returnvalue (Utilities|GetDataTableRow "/Game/Assets/DataTables/EvidenceDT/DT_LevelListEvidence.DT_LevelListEvidence" (Utilities|String|StringToName DT_LevelListEvidence))
      (:then
        (for _array_element (Utilities|Struct|BreakS_LevelListEvidence _returnvalue)
          (Utilities|Array|Add (Variables|Default|GetAllEvidenceList) (.Id (Utilities|Struct|BreakS_ListEvidenceItem _array_element)))
          (Class|IInventory|AddItem(Message) (HUD|GetHUD (Game|GetPlayerController 0)) _array_element))
        (for _array_element_2 (Variables|Default|GetAllEvidenceList)
          (Development|PrintString _array_element_2)))
      (:RowNotFound
        (Development|PrintString "GS_InGame RowNotFound")))))

(event EventRefreshList
  (params (List :type Array%20of%20Strings))
  (Variables|Default|SetEvidenceList List)
  (CallFunction|CheckList))

(fn ConstructionScript)