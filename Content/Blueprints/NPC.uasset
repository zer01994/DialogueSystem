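; NPC Blueprint for a talkable character whose dialogue runs through its NPC_AI controller.
; It copies its DialogueTree to that controller in both the construction script and BeginPlay.
; The Interaction event tells the controller to start dialogue, and SwitchCamera blends the first player's view to this NPC.
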(event EventBeginPlay
  (bind _asnpc_ai (Utilities|Casting|CastToNPC_AI (AI|GetAIController self)))
  (Variables|/Game/Blueprints/NPC_AI.NPC_AI_C|SetDialogueTree _asnpc_ai (Variables|Default|GetDialogueTree)))

(event Collision|EventActorBeginOverlap
  (params (OtherActor :type Actor%20Object%20Reference)))

(event EventTick
  (params (DeltaSeconds :type Float%20%28single-precision%29)))

(event EventInteraction
  (bind _asnpc_ai (Utilities|Casting|CastToNPC_AI (AI|GetAIController self)))
  (Default|StartDialogue _asnpc_ai))

(event EventSwitchCamera
  (Game|Player|SetViewTargetwithBlend (Game|GetPlayerController 0) self 0.0 "VTBlend_Linear" 0.0 false))

(fn ConstructionScript
  (bind _asnpc_ai (Utilities|Casting|CastToNPC_AI (AI|GetAIController self)))
  (Variables|/Game/Blueprints/NPC_AI.NPC_AI_C|SetDialogueTree _asnpc_ai (Variables|Default|GetDialogueTree)))